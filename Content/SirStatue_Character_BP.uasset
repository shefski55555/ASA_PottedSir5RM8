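; SirStatue character for the Potted Bots, adding a radial-menu category to set range, range visibility, task order and bot mode.
; BeginPlay reads game INI options to trim allowed bot modes; the menu builder moves surviving inherited mode entries into that category.
; Radius cycles through presets and feeds the AI blackboard alongside a self reference.
; RepNotifies scale the range visual and show it only to allied players while alive.
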(event EventPossessed
  (params (NewController :type Controller%20Object%20Reference))
  (|CallParentFunction NewController)
  (AI|Components|Blackboard|SetValueasObject (AI|GetBlackboard 0) (Utilities|Name|MakeLiteralName "NPCReference") self)
  (Class|BlackboardComponent|SetValueasInt (AI|GetBlackboard 0) (Utilities|Name|MakeLiteralName "Radius") (Variables|Default|GetRadius)))

(event Collision|EventActorBeginOverlap
  (params (OtherActor :type Actor%20Object%20Reference)))

(event EventTick
  (params (DeltaSeconds :type Float%20%28single-precision%29)))

(event EventDockingBayTryMultiUse
  (params (ForPC :type Player%20Controller%20Object%20Reference) (UseIndex :type Integer) (ForBay :type Primal%20Structure%20Object%20Reference))
  (|CallParentFunction ForPC UseIndex ForBay))

(event EventBPClientDoMultiUse
  (params (ForPC :type Player%20Controller%20Object%20Reference) (ClientUseIndex :type Integer))
  (bind _ranges (Variables|Default|GetRanges))
  (|CallParentFunction ForPC ClientUseIndex)
  (Utilities|FlowControl|Sequence
    (:then_1
      (if (== ClientUseIndex 13428)
        (Class|ShooterPlayerController|SetMultiUseWheelCategory (Class|PrimalAutocastFunctions|PCtoSPC ForPC) ClientUseIndex 0 0)
        (if (== ClientUseIndex 13429)
          (bind _output_get (Variables|Default|SetRadius self (Math|Integer|SelectInt (Utilities|Array|Get(acopy) _ranges) (Utilities|Array|Get(acopy) _ranges (+ (Utilities|Array|FindItem _ranges (Variables|Default|GetRadius)) 1)) (> (+ (Utilities|Array|FindItem _ranges (Variables|Default|GetRadius)) 1) (- (Utilities|Array|Length (Variables|Default|GetRanges)) 1))) false))
          (Class|BlackboardComponent|SetValueasInt (AI|GetBlackboard 0) (Utilities|Name|MakeLiteralName "Radius") _output_get))))))

(event EventOnSetDeath
  (|CallParentFunction)
  (Variables|Default|SetShowRange false true))

(event EventUnpossessed
  (params (OldController :type Controller%20Object%20Reference))
  (|CallParentFunction OldController)
  (Utilities|Array|Clear (Variables|Default|GetTaskList)))

(fn ConstructionScript
  (|CallParentFunction))

(fn BPGetMultiUseEntries
  (params (ForPC :type Player%20Controller%20Object%20Reference) (MultiUseEntries :type Array%20of%20Multi%20Use%20Entry%20Structures))
  (bind _radius (Variables|Default|GetRadius))
  (bind _ranges (Variables|Default|GetRanges))
  (bind _returnvalue (Utilities|Array|FindItem _ranges _radius))
  (bind _returnvalue_2 (|CallParentFunction ForPC MultiUseEntries))
  (Utilities|Array|Add _returnvalue_2 (Utilities|Struct|MakeMultiUseEntry 0 "Potted Bots" 13428 100 false false false false false false false false true false false true false false 0 false 123 "(B=175,G=175,R=175,A=255)" "(B=255,G=255,R=255,A=255)" 0.0 0.0 0 -1 -1 "/Sir-5r_Statue/Icons/Potted_Category.Potted_Category" "(B=255,G=255,R=255,A=255)" false false 0 13428))
  (Utilities|Array|Add _returnvalue_2 (Utilities|Struct|MakeMultiUseEntry 0 (Utilities|String|SelectString "Hide Range" "Show Range" (Variables|Default|GetShowRange)) 13430 100 false false false false false false false false true false false false false false 0 false 13428 "(B=175,G=175,R=175,A=255)" "(B=255,G=255,R=255,A=255)" 0.0 0.0 0 -1 -1 (select (Variables|Default|GetShowRange) (Variables|Default|GetHideRangeIcon) (Variables|Default|GetShowRangeIcon)) "(B=255,G=255,R=255,A=255)" true))
  (Utilities|Array|Add _returnvalue_2 (Utilities|Struct|MakeMultiUseEntry 0 (Utilities|String|Append "Change Range (" (Utilities|String|SelectString "Close" (Utilities|String|SelectString "Short" (Utilities|String|SelectString "Medium" (Utilities|String|SelectString "Far" (Utilities|String|SelectString "Very Far" "Like Really Really Far" (== _returnvalue 4)) (== _returnvalue 3)) (== _returnvalue 2)) (== _returnvalue 1)) (== _returnvalue 0)) ")") 13429 100 false false false false false false false false true false false false false false 0 false 13428 "(B=175,G=175,R=175,A=255)" "(B=255,G=255,R=255,A=255)" 0.0 0.0 0 -1 -1 "/Game/PrimalEarth/UI/UI_Final_Assets/RW/General/Range/RW_Adjust_Range.RW_Adjust_Range" "(B=255,G=255,R=255,A=255)" true))
  (Utilities|Array|Add _returnvalue_2 (Utilities|Struct|MakeMultiUseEntry 0 (Utilities|String|SelectString "Custom Task Order" "Vanilla Task Order" (Variables|Default|GetUseCustomSorting)) 13431 100 false false false false false false false false true false false false false false 0 false 13428 "(B=175,G=175,R=175,A=255)" "(B=255,G=255,R=255,A=255)" 0.0 0.0 0 -1 -1 (select (Variables|Default|GetUseCustomSorting) "/Sir-5r_Statue/Icons/Icon_Sorted.Icon_Sorted" "/Sir-5r_Statue/Icons/Icon_Unsort.Icon_Unsort") "(B=255,G=255,R=255,A=255)" true))
  (Utilities|FlowControl|Sequence
    (:then_0
      (bind _array_element (Utilities|Array|ForEachLoopwithBreak _returnvalue_2)
        (:LoopBody
          (LocalVariables|SetModeRemoved true)
          (bind _array_element_2 (Utilities|Array|ForEachLoopwithBreak (Variables|Default|GetAllowedBotModes) :!label _label)
            (:LoopBody
              (Utilities|FlowControl|Sequence
                (:then_0
                  (if (and (Utilities|Enum|Equal(Enum) (.UseString (Utilities|Struct|BreakMultiUseEntry _array_element)) "potted butler") (Utilities|Enum|Equal(Enum) _array_element_2 "PottedButler"))
                    (LocalVariables|SetModeRemoved false :!label _label_2)
                    (goto _label Break)))
                (:then_1
                  (if (and (Utilities|Enum|Equal(Enum) (.UseString (Utilities|Struct|BreakMultiUseEntry _array_element)) "potted butler (slow)") (Utilities|Enum|Equal(Enum) _array_element_2 "PottedButlerSlow"))
                    (goto _label_2)))
                (:then_2
                  (if (and (Utilities|Enum|Equal(Enum) (.UseString (Utilities|Struct|BreakMultiUseEntry _array_element)) "potted repair") (Utilities|Enum|Equal(Enum) _array_element_2 "PottedRepair"))
                    (goto _label_2)))
                (:then_3
                  (if (and (Utilities|Enum|Equal(Enum) (.UseString (Utilities|Struct|BreakMultiUseEntry _array_element)) "potted harvest") (Utilities|Enum|Equal(Enum) _array_element_2 "PottedHarvest"))
                    (goto _label_2)))))
            (:Completed
              (if (Math|Boolean|ANDBoolean (> (.UseIndex (Utilities|Struct|BreakMultiUseEntry _array_element)) 1053) (< (.UseIndex (Utilities|Struct|BreakMultiUseEntry _array_element)) 1100) (== (.WheelCategory (Utilities|Struct|BreakMultiUseEntry _array_element)) 123) (not (LocalVariables|GetModeRemoved)))
                (Utilities|Array|Add (LocalVariables|GetTempList) (Utilities|Struct|MakeMultiUseEntry 0 (.UseString (Utilities|Struct|BreakMultiUseEntry _array_element)) (.UseIndex (Utilities|Struct|BreakMultiUseEntry _array_element)) (.Priority (Utilities|Struct|BreakMultiUseEntry _array_element)) false false false false false false false false false false false false false false 0 false 13428 "(B=175,G=175,R=175,A=255)" "(B=255,G=255,R=255,A=255)" 0.0 0.0 0 -1 -1 (.Icon (Utilities|Struct|BreakMultiUseEntry _array_element))))))))))
    (:then_1
      (LocalVariables|SetTempList_2 _returnvalue_2)
      (bind _array_element_3 (Utilities|Array|ForEachLoopwithBreak _returnvalue_2)
        (:LoopBody
          (if (Math|Boolean|ANDBoolean true (> (.UseIndex (Utilities|Struct|BreakMultiUseEntry _array_element_3)) 1053) (< (.UseIndex (Utilities|Struct|BreakMultiUseEntry _array_element_3)) 1100) true (== (.WheelCategory (Utilities|Struct|BreakMultiUseEntry _array_element_3)) 123))
            (Utilities|Array|RemoveItem (LocalVariables|GetTempList_2) _array_element_3)))))
    (:then_2
      (Utilities|Array|AppendArray (LocalVariables|GetTempList_2) (LocalVariables|GetTempList))
      (return (LocalVariables|GetTempList_2)))))

(fn ReceiveBeginPlay
  (|CallParentFunction)
  (Utilities|FlowControl|Sequence
    (:then_0
      (bind _asshooter_game_mode (Utilities|Casting|CastToShooterGameMode (Game|GetGameMode)))
      (Class|ShooterGameMode|InitOptionBool _asshooter_game_mode "" "Potted S1R5RM8" "PottedButler" true)
      (Class|ShooterGameMode|InitOptionBool _asshooter_game_mode "" "Potted S1R5RM8" "PottedButlerSlow" true)
      (Class|ShooterGameMode|InitOptionBool _asshooter_game_mode "" "Potted S1R5RM8" "PottedRepair" true)
      (Class|ShooterGameMode|InitOptionBool _asshooter_game_mode "" "Potted S1R5RM8" "PottedHarvest" true)
      (Class|ShooterGameMode|InitOptionFloat _asshooter_game_mode "" "Potted S1R5RM8" "MinWindTurbineRepairHealthPercent" 0.5)
      (Utilities|FlowControl|Sequence
        (:then_0
          (bind _returnvalue (Class|ShooterGameMode|GetBoolOptionIni _asshooter_game_mode "Potted S1R5RM8" "PottedButler" true))
          (if (not _returnvalue)
            (Utilities|Array|RemoveItem (Variables|Default|GetAllowedBotModes) "PottedButler")))
        (:then_1
          (bind _returnvalue_2 (Class|ShooterGameMode|GetBoolOptionIni _asshooter_game_mode "Potted S1R5RM8" "PottedButlerSlow" true))
          (if (not _returnvalue_2)
            (Utilities|Array|RemoveItem (Variables|Default|GetAllowedBotModes) "PottedButlerSlow")))
        (:then_2
          (bind _returnvalue_3 (Class|ShooterGameMode|GetBoolOptionIni _asshooter_game_mode "Potted S1R5RM8" "PottedRepair" true))
          (if (not _returnvalue_3)
            (Utilities|Array|RemoveItem (Variables|Default|GetAllowedBotModes) "PottedRepair")))
        (:then_3
          (bind _returnvalue_4 (Class|ShooterGameMode|GetBoolOptionIni _asshooter_game_mode "Potted S1R5RM8" "PottedHarvest" true))
          (if (not _returnvalue_4)
            (Utilities|Array|RemoveItem (Variables|Default|GetAllowedBotModes) "PottedHarvest")))
        (:then_4
          (Utilities|IsValid (Variables|Default|GetMyAIData)
            (:Is%20Not%20Valid
              (bind _returnvalue_5 (Game|ConstructObjectfromClass "/Game/Packs/Steampunk/Dinos/HelperBot/AI/BP_HelperBot_AIData.BP_HelperBot_AIData_C"))
              (Variables|Default|SetMyAIData _returnvalue_5)
              (Development|PrintString 0 "SET AI DATA" true true "(R=1.000000,G=0.000000,B=0.073311,A=1.000000)" 5.0))))))
    (:then_1
      (Class|ShooterGameMode|InitOptionBool _asshooter_game_mode "" "Potted S1R5RM8" "CropFertFix" false)
      (bind _returnvalue_6 (Class|ShooterGameMode|GetBoolOptionIni _asshooter_game_mode "Potted S1R5RM8" "CropFertFix" false))
      (Variables|Default|SetCropFertFix _returnvalue_6 false))))

(fn BPTryMultiUse
  (params (ForPC :type Player%20Controller%20Object%20Reference) (UseIndex :type Integer))
  (bind _ranges (Variables|Default|GetRanges))
  (bind _returnvalue (|CallParentFunction ForPC UseIndex))
  (Utilities|FlowControl|Sequence
    (:then_0
      (if (== UseIndex 13429)
        (bind _output_get (Variables|Default|SetRadius self (Math|Integer|SelectInt (Utilities|Array|Get(acopy) _ranges) (Utilities|Array|Get(acopy) _ranges (+ (Utilities|Array|FindItem _ranges (Variables|Default|GetRadius)) 1)) (> (+ (Utilities|Array|FindItem _ranges (Variables|Default|GetRadius)) 1) (- (Utilities|Array|Length (Variables|Default|GetRanges)) 1))) false))
        (Class|BlackboardComponent|SetValueasInt (AI|GetBlackboard 0) (Utilities|Name|MakeLiteralName "Radius") _output_get)
        (return _returnvalue)))
    (:then_1
      (if (== UseIndex 13430)
        (Variables|Default|SetShowRange (not (Variables|Default|GetShowRange)) true)))
    (:then_2
      (if (== UseIndex 13431)
        (Development|PrintString 0)
        (Variables|Default|SetUseCustomSorting (not (Variables|Default|GetUseCustomSorting)) false)))))

(fn OnRepShowRange
  (bind _radius (Variables|Default|GetRadius))
  (bind _radiusvisual (Variables|Default|GetRadiusVisual))
  (bind _returnvalue (Math|Conversions|ToFloat(Integer) _radius))
  (Class|KismetSystemLibrary|CanRunCosmeticEvents
    (:Yes
      (bind _asprimal_character (Utilities|Casting|CastToPrimalCharacter (Pawn|GetControlledPawn (Game|GetPlayerController 0))))
      (bind _returnvalue_2 (Class|PrimalCharacter|IsAlliedwithOtherTeam _asprimal_character (Variables|Default|GetTargetingTeam)))
      (Transformation|SetWorldScale3D _radiusvisual (Math|Vector|MakeVector _returnvalue _returnvalue _returnvalue))
      (Rendering|SetVisibility _radiusvisual (Math|Boolean|ANDBoolean (Variables|Default|GetShowRange) _returnvalue_2 (not (Class|PrimalActor|IsDead))) true))))

(fn OnRepRadius
  (bind _radius (Variables|Default|GetRadius))
  (bind _returnvalue (Math|Conversions|ToFloat(Integer) _radius))
  (Transformation|SetWorldScale3D (Variables|Default|GetRadiusVisual) (Math|Vector|MakeVector _returnvalue _returnvalue _returnvalue)))

(fn OnRepUseCustomSorting)